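; BP_Spawn_Nourriture is a spawner actor, named for food, that keeps respawning a pickupable item.
; It spawns the configured Item class at its root component's transform on BeginPlay.
; When an actor tagged Pickupable stops overlapping its Box, it waits a short delay and spawns another Item.
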(event `self.ReceiveBeginPlay`
  (`self.Spawn Item`))

(event `Spawn Item`
  (`|SpawnActorFromClass` (`self.Item`) (`SceneComponent.GetRelativeTransform` (`self.DefaultSceneRoot`)) "Undefined" "MultiplyWithRoot" null null))

(event `self.Box.OnComponentEndOverlap`
  (params (OverlappedComponent :type "PrimitiveComponent Object Reference") (OtherActor :type "Actor Object Reference") (OtherComp :type "PrimitiveComponent Object Reference") (OtherBodyIndex :type Integer))
  (if (`self.ActorHasTag` OtherActor "Pickupable")
    (`KismetSystemLibrary.Delay` 3.0)
    (`self.Spawn Item`)))

(fn `UserConstructionScript`)