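; BP_Items is an item actor that tracks whether it can be taken through a CanTake flag.
; Trigger begin and end overlap events search overlapping BP_Player actors for the "Hand" tag, setting the flag true or false respectively.
; The end event clears the flag only if such an actor is still found overlapping.
; Tick prints CanTake every frame, and no pickup action is implemented here.
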(event `self.ReceiveTick`
  (params (DeltaSeconds :type "Float (single-precision)"))
  (`KismetSystemLibrary.PrintString` (`KismetStringLibrary.Conv_BoolToString` (`self.CanTake`)) true true (struct :`R` 1.0 :`G` 0.15379 :`A` 1.0) 0.0))

(event `self.Trigger.OnComponentBeginOverlap`
  (params (OverlappedComponent :type "PrimitiveComponent Object Reference") (OtherActor :type "Actor Object Reference") (OtherComp :type "PrimitiveComponent Object Reference") (OtherBodyIndex :type Integer) (bFromSweep :type Boolean) (SweepResult :type "HitResult Structure (by ref)"))
  (for _array_element (`self.GetOverlappingActors` "/Game/Characters/BP_Player.BP_Player_C")
    (if (`self.ActorHasTag` _array_element "Hand")
      (set `self.CanTake` true))))

(event `self.Trigger.OnComponentEndOverlap`
  (params (OverlappedComponent :type "PrimitiveComponent Object Reference") (OtherActor :type "Actor Object Reference") (OtherComp :type "PrimitiveComponent Object Reference") (OtherBodyIndex :type Integer))
  (for _array_element (`self.GetOverlappingActors` "/Game/Characters/BP_Player.BP_Player_C")
    (if (`self.ActorHasTag` _array_element "Hand")
      (set `self.CanTake` false))))

(fn `UserConstructionScript`)