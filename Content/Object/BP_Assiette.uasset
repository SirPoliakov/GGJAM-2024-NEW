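; BP_Assiette is a plate that snaps food items onto itself to assemble a dish of mussels, fries and sauce.
; When its Trigger is overlapped, each overlapping BP_Items tagged Pickupable fires SetIngerdient, which runs PlaceIngerdient on every overlapping item, tagged Pickupable or not.
; PlaceIngerdient uses the item's tag to attach it to the matching Assiette socket, snapping location and rotation while keeping world scale.
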(event `self.Trigger.OnComponentBeginOverlap`
  (params (OverlappedComponent :type "PrimitiveComponent Object Reference") (OtherActor :type "Actor Object Reference") (OtherComp :type "PrimitiveComponent Object Reference") (OtherBodyIndex :type Integer) (bFromSweep :type Boolean) (SweepResult :type "HitResult Structure (by ref)"))
  (for _array_element (`self.GetOverlappingActors` "/Game/Object/BP_Items.BP_Items_C")
    (if (`self.ActorHasTag` _array_element "Pickupable")
      (`self.Set Ingerdient`))))

(event `Set Ingerdient`
  (for _array_element (`self.GetOverlappingActors` "/Game/Object/BP_Items.BP_Items_C")
    (if (`self.ActorHasTag` _array_element "Moules")
      (`self.K2_AttachToComponent` _array_element (`self.Assiette`) "Moules" "SnapToTarget" "SnapToTarget" "KeepWorld" true)
      (elif (`self.ActorHasTag` _array_element "Frits")
        (`self.K2_AttachToComponent` _array_element (`self.Assiette`) "Frits" "SnapToTarget" "SnapToTarget" "KeepWorld" true)
        (elif (`self.ActorHasTag` _array_element "Sauce")
          (`self.K2_AttachToComponent` _array_element (`self.Assiette`) "Sauce" "SnapToTarget" "SnapToTarget" "KeepWorld" true))))))

(fn `UserConstructionScript`)