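; BP_Player is the player character, providing limited-angle camera look and a toggle to take or drop an item.
; BeginPlay adds the Enhanced Input mapping context, then NewMacro clamps camera pitch and yaw, with each sequence branch exiting to re-cache a single BP_Items actor found by class.
; Look inputs drive controller yaw and pitch.
; IA_Take alternates TakeItems and DropsItems on that cached actor through a FlipFlop.
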(event `self.ReceiveBeginPlay`
  (bind _asbp_player_controlleur (cast `/Game/Characters/BP_PlayerControlleur` (`self.GetController`)))
  (bind _returnvalue (pcsubsystem `EnhancedInputLocalPlayerSubsystem` _asbp_player_controlleur))
  (`/Engine/EditorBlueprintResources/StandardMacros.IsValid` _returnvalue
    (:`Is Valid`
      (`EnhancedInputSubsystemInterface.AddMappingContext` _returnvalue "/Game/Input/IMC_Player.IMC_Player" 0 (struct))
      (`self.NewMacro`
        (:`OUT`
          (bind _returnvalue_2 (`GameplayStatics.GetActorOfClass` "/Game/Object/BP_Items.BP_Items_C"))
          (set `self.BP_Tiems` _returnvalue_2))))))

(event `EnhancedInput|/Game/Input/IA_LookYaw`
  (params (ActionValue :type "Float (double-precision)") (ElapsedSeconds :type "Float (double-precision)") (TriggeredSeconds :type "Float (double-precision)") (InputAction :type "InputAction Object Reference" :default "/Game/Input/IA_LookYaw.IA_LookYaw"))
  ;[1 1 1] Look At Camera
  (:`Triggered`
    (`self.AddControllerYawInput` ActionValue)))

(event `EnhancedInput|/Game/Input/IA_LookPitch`
  (params (ActionValue :type "Float (double-precision)") (ElapsedSeconds :type "Float (double-precision)") (TriggeredSeconds :type "Float (double-precision)") (InputAction :type "InputAction Object Reference" :default "/Game/Input/IA_LookPitch.IA_LookPitch"))
  ;[1 1 1] Look At Camera
  (:`Triggered`
    (`self.AddControllerPitchInput` ActionValue)))

(event `EnhancedInput|/Game/Input/IA_Take`
  (params (ActionValue :type Boolean) (ElapsedSeconds :type "Float (double-precision)") (TriggeredSeconds :type "Float (double-precision)") (InputAction :type "InputAction Object Reference" :default "/Game/Input/IA_Take.IA_Take"))
  (bind _bp_tiems (`self.BP_Tiems`))
  (:`Completed`
    (`/Engine/EditorBlueprintResources/StandardMacros.FlipFlop`
      (:`A`
        (`/Game/Object/BP_Items.Take Items` _bp_tiems))
      (:`B`
        (`/Game/Object/BP_Items.Drops Items` _bp_tiems)))))

(fn `UserConstructionScript`)