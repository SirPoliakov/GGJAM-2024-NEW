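; Player controller for the main menu that handles play, credits, quit and back through Enhanced Input.
; On BeginPlay it adds the menu mapping context and caches the GM_Menus game mode, which holds the menu and credits widget references.
; Play loads L_Main_Level and Quit exits, while an IsCreditsOpen flag blocks those actions during credits and lets Back swap the widgets back.
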(event `self.ReceiveBeginPlay`
  (`EnhancedInputSubsystemInterface.AddMappingContext` (pcsubsystem `EnhancedInputLocalPlayerSubsystem` self) "/Game/Input/IMC/IMPC_Menu.IMPC_Menu" 0 (struct))
  (bind _asgm_menus (cast `/Game/Blueprint/GM_Menus` (`GameplayStatics.GetGameMode`)))
  (set `self.As GM Menus` _asgm_menus))

(event `EnhancedInput|/Game/Input/IA/Menus/IA_Play`
  (params (ActionValue :type Boolean) (ElapsedSeconds :type "Float (double-precision)") (TriggeredSeconds :type "Float (double-precision)") (InputAction :type "InputAction Object Reference" :default "/Game/Input/IA/Menus/IA_Play.IA_Play"))
  (:`Started`
    (if (not (`self.isCreditsOpen`))
      (`GameplayStatics.OpenLevel` "L_Main_Level"))))

(event `EnhancedInput|/Game/Input/IA/Menus/IA_Credits`
  (params (ActionValue :type Boolean) (ElapsedSeconds :type "Float (double-precision)") (TriggeredSeconds :type "Float (double-precision)") (InputAction :type "InputAction Object Reference" :default "/Game/Input/IA/Menus/IA_Credits.IA_Credits"))
  (bind _as_gm_menus (`self.As GM Menus`))
  (:`Started`
    (if (not (`self.isCreditsOpen`))
      (set `self.isCreditsOpen` true)
      (`Widget.RemoveFromParent` (`/Game/Blueprint/GM_Menus.WB Menu Ref` _as_gm_menus))
      (`UserWidget.AddToViewport` (`/Game/Blueprint/GM_Menus.WB Credits Ref` _as_gm_menus) 0))))

(event `EnhancedInput|/Game/Input/IA/Menus/IA_Quit`
  (params (ActionValue :type Boolean) (ElapsedSeconds :type "Float (double-precision)") (TriggeredSeconds :type "Float (double-precision)") (InputAction :type "InputAction Object Reference" :default "/Game/Input/IA/Menus/IA_Quit.IA_Quit"))
  (:`Started`
    (if (not (`self.isCreditsOpen`))
      (`KismetSystemLibrary.QuitGame` null "Quit"))))

(event `EnhancedInput|/Game/Input/IA/Menus/IA_Back`
  (params (ActionValue :type Boolean) (ElapsedSeconds :type "Float (double-precision)") (TriggeredSeconds :type "Float (double-precision)") (InputAction :type "InputAction Object Reference" :default "/Game/Input/IA/Menus/IA_Back.IA_Back"))
  (bind _as_gm_menus (`self.As GM Menus`))
  (:`Triggered`
    (if (`self.isCreditsOpen`)
      (set `self.isCreditsOpen` false)
      (`Widget.RemoveFromParent` (`/Game/Blueprint/GM_Menus.WB Credits Ref` _as_gm_menus))
      (`UserWidget.AddToViewport` (`/Game/Blueprint/GM_Menus.WB Menu Ref` _as_gm_menus) 0))))

(fn `UserConstructionScript`)