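; BP_Client is an order-placing client with a patience bar, owned by BP_OrderManager.
; On BeginPlay it pulls a random client type and order from the manager, then a looping timer raises patience and updates WBP_ClientBar until the maximum.
; ChangeClientState swaps the LynxTexture material from a state DataTable row, using the same table for all three animal types.
; ExplodeClient only stops the timer.
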(event `self.ReceiveBeginPlay`
  (bind _asbp_order_manager (cast `/Game/Blueprint/Orders/BP_OrderManager` (`self.GetOwner`)))
  (bind _client (`/Game/Blueprint/Orders/BP_OrderManager.GetRandomClient` _asbp_order_manager))
  (set `self.Client Type` _client)
  (bind _order (`/Game/Blueprint/Orders/BP_OrderManager.GetRandomOrder` _asbp_order_manager))
  (set `self.CurrentOrder` _order)
  (bind _returnvalue (`KismetSystemLibrary.K2_SetTimerDelegate` (delegate `RaisePatience`) 0.05 true))
  (set `self.PatienceTimer` _returnvalue)
  (bind _aswbp_client_bar (cast `/Game/Blueprint/Widget/WBP_ClientBar` (`WidgetComponent.GetWidget` (`self.Widget`))))
  (set `self.ClientBar` _aswbp_client_bar))

(event `RaisePatience`
  (`self.ChangeMood`))

(fn `ChangeClientState`
  (params (`New State` :type "/Game/Blueprint/Orders/E_ClientState Enum" :default "NewEnumerator0"))
  (set `self.ClientState` `New State`)
  (switch `/Game/Blueprint/Orders/E_ClientType` (`self.Client Type`)
    (:`NewEnumerator0`
      (set `self.CurrentDataTable` "/Game/Blueprint/Orders/DT_Client_State.DT_Client_State"))
    (:`NewEnumerator1`
      (set `self.CurrentDataTable` "/Game/Blueprint/Orders/DT_Client_State.DT_Client_State"))
    (:`NewEnumerator2`
      (set `self.CurrentDataTable` "/Game/Blueprint/Orders/DT_Client_State.DT_Client_State")))
  (bind _returnvalue (`|GetDataTableRow` (`self.CurrentDataTable`) (`|GetEnumeratorName` (`self.ClientState`)))
    (:`then`
      (`PrimitiveComponent.SetMaterial` (`self.LynxTexture`) 0 (`.LynxTexture_17_213BC2F34AB572FF72C2E0A8FAB2B6E1` (break `/Game/Blueprint/Orders/S_ClientState` _returnvalue))))))

(fn `ChangeMood`
  (bind _current_patience (`self.Current Patience`))
  (set `self.Current Patience` (+ _current_patience 0.05))
  (if (not (>= _current_patience (`self.MaxPatience`)))
    (`self.SetPercent`)))

(fn `ExplodeClient`
  (`KismetSystemLibrary.K2_ClearAndInvalidateTimerHandle` (`self.PatienceTimer`)))

(fn `SetPercent`
  (set `/Game/Blueprint/Widget/WBP_ClientBar.CurrentPatience` (/ (`self.Current Patience`) (`self.MaxPatience`)) (`self.ClientBar`)))

(fn `UserConstructionScript`)