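; Order manager that spawns clients at slots on randomized timers and provides their food orders of fries, mussels and sauce.
; Loads order and client data tables at start, then picks orders, clients and spawn delays by cumulative-probability weighted random.
; Clients take a random free slot, or a waiting flag triggers a spawn when one is removed.
; CheckOrder validates each ingredient, clears it from the order and reports completion.
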(event `self.ReceiveBeginPlay`
  (`self.SetupOrderList`
    (:`Completed`
      (`self.SetupClientList`
        (:`Completed`
          (bind _returnvalue (`KismetSystemLibrary.K2_SetTimerDelegate` (delegate `SpawnClientEvent`) (`self.firstClientDelay`)))
          (set `self.EventClientSpawnHandle` _returnvalue))))))

(event `SpawnClientEvent`
  (`self.SpawnClient`)
  (bind _time_to_wait (`self.GetRandomTime`))
  (`KismetSystemLibrary.K2_ClearAndInvalidateTimerHandle` (`self.EventClientSpawnHandle`))
  (bind _returnvalue (`KismetSystemLibrary.K2_SetTimerDelegate` (delegate `SpawnClientEvent`) _time_to_wait))
  (set `self.EventClientSpawnHandle` _returnvalue))

(fn `CheckOrder`
  (params (CurrentOrder :type "/Game/Blueprint/Orders/S_OrderContentData Structure") (FoodPutIn :type "/Game/Blueprint/Orders/E_FoodType Enum" :default "NewEnumerator0"))
  (returns (`Current Order` :type "/Game/Blueprint/Orders/S_OrderContentData Structure") (IsCorrect :type Boolean) (OrderFinished :type Boolean))
  (locals (isCorrectIngredient :type Boolean) (isFinished :type Boolean) (order :type "/Game/Blueprint/Orders/S_OrderContentData Structure"))
  (bind (_order_hasfries _order_hasmussels _order_hassauce) (break `/Game/Blueprint/Orders/S_OrderContentData` (`local.order`)))
  (bind (_order_hasfries_2 _order_hasmussels_2 _order_hassauce_2) (break `/Game/Blueprint/Orders/S_OrderContentData` (`local.order`)))
  (bind (_order_hasfries_3 _order_hasmussels_3 _order_hassauce_3) (break `/Game/Blueprint/Orders/S_OrderContentData` (`local.order`)))
  (set `local.order` CurrentOrder)
  (switch `/Game/Blueprint/Orders/E_FoodType` FoodPutIn
    (:`NewEnumerator0`
      (if _order_hasfries
        (set `local.isCorrectIngredient` true :!label _label)
        (set `local.order` (make `/Game/Blueprint/Orders/S_OrderContentData` (xor (`|EnumEquality` FoodPutIn "NewEnumerator0") _order_hasfries_3) (xor (`|EnumEquality` FoodPutIn "NewEnumerator1") _order_hasmussels_3) (xor (`|EnumEquality` FoodPutIn "NewEnumerator2") _order_hassauce_3) null))
        (bind _output_get (set `local.isFinished` (and (not _order_hasfries_2) (not _order_hasmussels_2) (not _order_hassauce_2))))))
    (:`NewEnumerator1`
      (if _order_hasmussels
        (goto _label)
        (else
          _)))
    (:`NewEnumerator2`
      (if _order_hassauce
        (goto _label)
        (else
          _))))
  (return (`local.order`) (`local.isCorrectIngredient`) _output_get))

(fn `GetRandomClient`
  (returns (Client :type "/Game/Blueprint/Orders/E_ClientType Enum"))
  (locals (PercentSelected :type "Float (double-precision)") (Percent :type "Array of Float (double-precision)") (OrderID :type Integer))
  (bind _possibleclients (`self.possibleClients`))
  (bind _percent (`local.Percent`))
  (bind _percent_2 (`local.Percent`))
  (bind _percent_3 (`local.Percent`))
  (bind _output_client (break `/Game/Blueprint/Orders/S_ClientProbability` (`|GetArrayItem` _possibleclients (`local.OrderID`))))
  (for (_array_element _array_index) _possibleclients
    (if (== _array_index 0)
      (bind (_client _probability) (break `/Game/Blueprint/Orders/S_ClientProbability` _array_element))
      (`KismetArrayLibrary.Array_Add` _percent_2 _probability)
      (else
        (`KismetArrayLibrary.Array_Add` _percent_2 (+ _probability (`|GetArrayItem` _percent (`KismetArrayLibrary.Array_LastIndex` _percent)))))))
  (set `local.PercentSelected` (`KismetMathLibrary.RandomFloatInRange` 0.0 (`|GetArrayItem` _percent_3 (`KismetArrayLibrary.Array_LastIndex` _percent_3))))
  (for (_array_element_2 _array_index_2) (`local.Percent`)
    (if (< _array_element_2 (`local.PercentSelected`))
      (set `local.OrderID` (+ 1 _array_index_2))))
  (return _output_client))

(fn `GetRandomOrder`
  (returns (Order :type "/Game/Blueprint/Orders/S_OrderContentData Structure"))
  (locals (Percent :type "Array of Float (double-precision)") (PercentSelected :type "Float (double-precision)") (OrderID :type Integer))
  (bind _percent (`local.Percent`))
  (bind _percent_2 (`local.Percent`))
  (bind _percent_3 (`local.Percent`))
  (bind _possibleorders (`self.possibleOrders`))
  (bind _output_content (break `/Game/Blueprint/Orders/S_OrderProbability` (`|GetArrayItem` _possibleorders (`local.OrderID`))))
  (for (_array_element _array_index) _possibleorders
    (if (== _array_index 0)
      (bind (_content _probability) (break `/Game/Blueprint/Orders/S_OrderProbability` _array_element))
      (`KismetArrayLibrary.Array_Add` _percent _probability)
      (else
        (`KismetArrayLibrary.Array_Add` _percent (+ _probability (`|GetArrayItem` _percent_2 (`KismetArrayLibrary.Array_LastIndex` _percent_2)))))))
  (set `local.PercentSelected` (`KismetMathLibrary.RandomFloatInRange` 0.0 (`|GetArrayItem` _percent_3 (`KismetArrayLibrary.Array_LastIndex` _percent_3))))
  (for (_array_element_2 _array_index_2) (`local.Percent`)
    (if (< _array_element_2 (`local.PercentSelected`))
      (set `local.OrderID` (+ 1 _array_index_2))
      (else
        (break))))
  (return _output_content))

(fn `GetRandomPlace`
  (returns (SlotID :type Integer))
  (locals (CurrentPlace :type Integer :default -1))
  (bind _nmaxclient (`self.nMaxClient`))
  (bind _returnvalue (`KismetMathLibrary.RandomIntegerInRange` 0 _nmaxclient))
  (for _index (range _returnvalue (+ (+ _nmaxclient _returnvalue) 1))
    (bind _returnvalue_2 (mod _index _nmaxclient))
    (if (== (`|GetArrayItem` (`self.CurrentClient`) _returnvalue_2) null)
      (set `local.CurrentPlace` _returnvalue_2)
      (break)))
  (return (`local.CurrentPlace`)))

(fn `GetRandomTime`
  (returns (`Time to Wait` :type "Float (double-precision)"))
  (locals (Percent :type "Array of Float (double-precision)") (PercentSelected :type "Float (double-precision)") (OrderID :type Integer))
  (bind _timespawnprob (`self.TimeSpawnProb`))
  (bind _timespawnprob_2 (`self.TimeSpawnProb`))
  (bind _percent (`local.Percent`))
  (bind _percent_2 (`local.Percent`))
  (bind _outrownames (`DataTableFunctionLibrary.GetDataTableRowNames` _timespawnprob))
  (for _array_element _outrownames
    (bind _returnvalue (`|GetDataTableRow` _timespawnprob _array_element)
      (:`then`
        (if (== (`KismetArrayLibrary.Array_Length` _percent) 0)
          (bind (_timetospawnmin _timetospawnmax _probability) (break `/Game/Blueprint/Orders/S_TimeSpawnProb` _returnvalue))
          (`KismetArrayLibrary.Array_Add` _percent _probability)
          (else
            (`KismetArrayLibrary.Array_Add` _percent (+ _probability (`|GetArrayItem` _percent (`KismetArrayLibrary.Array_LastIndex` _percent)))))))))
  (set `local.PercentSelected` (`KismetMathLibrary.RandomFloatInRange` 0.0 (`|GetArrayItem` _percent_2 (`KismetArrayLibrary.Array_LastIndex` _percent_2))))
  (for (_array_element_2 _array_index) (`local.Percent`)
    (if (< _array_element_2 (`local.PercentSelected`))
      (set `local.OrderID` (+ 1 _array_index))))
  (bind _outrownames_2 (`DataTableFunctionLibrary.GetDataTableRowNames` _timespawnprob_2))
  (bind _returnvalue_2 (`|GetDataTableRow` _timespawnprob_2 (`|GetArrayItem` _outrownames_2 (`local.OrderID`)))
    (:`then`
      (bind (_timetospawnmin_2 _timetospawnmax_2) (break `/Game/Blueprint/Orders/S_TimeSpawnProb` _returnvalue_2))
      (return (`KismetMathLibrary.RandomFloatInRange` _timetospawnmin_2 _timetospawnmax_2)))))

(fn `OrderToString`
  (params (`Order In` :type "/Game/Blueprint/Orders/S_OrderContentData Structure"))
  (returns (Out :type String))
  (return (`KismetStringLibrary.Concat_StrStr` "Fries : " (`KismetStringLibrary.Conv_BoolToString` `Order In_HasFries_3_55FBE9E845582700458B85A19DB9A71B`) " | Mussel : " (`KismetStringLibrary.Conv_BoolToString` `Order In_HasMussels_5_E66F90E24D1A4400C10CFEB011C50728`) " | Sauce : " (`KismetStringLibrary.Conv_BoolToString` `Order In_HasSauce_7_72CBA6CA4764623FDEA5A4AEB3493519`))))

(fn `RemoveClient`
  (params (ClientToRemove :type "/Game/Blueprint/Orders/BP_Client Object Reference"))
  (`KismetArrayLibrary.Array_RemoveItem` (`self.CurrentClient`) ClientToRemove)
  (if (`self.ClientWaiting`)
    (set `self.ClientWaiting` false)
    (`self.SpawnClientEvent`)))

(fn `SpawnClient`
  (bind _slotid (`self.GetRandomPlace`))
  (if (!= _slotid -1)
    (bind _returnvalue (`|SpawnActorFromClass` "/Game/Blueprint/Orders/BP_Client.BP_Client_C" (`self.GetTransform` (`|GetArrayItem` (`self.clientSlots`) _slotid)) "Undefined" "MultiplyWithRoot" self null))
    (`KismetArrayLibrary.Array_Set` (`self.CurrentClient`) _slotid _returnvalue)
    (else
      (set `self.ClientWaiting` true))))

(fn `UserConstructionScript`)