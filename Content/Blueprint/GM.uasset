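; GM sets up a two-player local game with a left and a right pawn, and starts the game's sound on BeginPlay.
; Each pawn's load event triggers possession: player controller 0 takes the left pawn, and a newly created local player takes the right.
; The right pawn's event then passes each pawn a reference to the other, relying on the left pawn having loaded first.
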(event `self.ReceiveBeginPlay`
  (`GameplayStatics.PlaySound2D` "/Game/Sounds/Musics/SC_CountryGame_Sound.SC_CountryGame_Sound" 1.0 1.0 0.0 null null))

(event `/Game/Blueprint/BPI_Comm.LPawnIstanceLoad`
  (params (LeftPawn :type "/Game/Blueprint/LeftPawn Object Reference"))
  (set `self.Left Pawn` LeftPawn)
  (`Controller.Possess` (`GameplayStatics.GetPlayerController` 0) LeftPawn))

(event `/Game/Blueprint/BPI_Comm.RPawnIstanceLoad`
  (params (RightPawn :type "/Game/Blueprint/RightPawn Object Reference"))
  (bind _left_pawn (`self.Left Pawn`))
  (bind _returnvalue (`GameplayStatics.CreatePlayer` -1))
  (`Controller.Possess` _returnvalue RightPawn)
  (message `/Game/Blueprint/BPI_Comm.RPawnIstanceLoad` _left_pawn RightPawn)
  (message `/Game/Blueprint/BPI_Comm.LPawnIstanceLoad` RightPawn _left_pawn))

(fn `UserConstructionScript`)