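; RightPawn is the right paw that grabs and drops items, coordinating with LeftPawn through overlap messages.
; Taking attaches the item to the paw's Hand socket and disables its physics and the paw's collision; releasing simulates physics for a short timer before freezing it and resetting.
; A reversible timeline drives the paw's grab morph target.
; Taking a beer-type item raises the GameMode's alcohol bar and spawns one of three escalating drunk post-process actors.
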(event `/Game/Blueprint/BPI_Comm.LPawnIstanceLoad`
  (params (LeftPawn :type "/Game/Blueprint/LeftPawn Object Reference"))
  (set `self.LeftPawn` LeftPawn))

(event `self.Triger Main.OnComponentBeginOverlap`
  (params (OverlappedComponent :type "PrimitiveComponent Object Reference") (OtherActor :type "Actor Object Reference") (OtherComp :type "PrimitiveComponent Object Reference") (OtherBodyIndex :type Integer) (bFromSweep :type Boolean) (SweepResult :type "HitResult Structure (by ref)"))
  (message `/Game/Blueprint/BPI_Comm.RightCanTake` (`self.LeftPawn`))
  (message `/Game/Blueprint/BPI_Item.GoToRef` OtherActor self))

(event `/Game/Blueprint/BPI_Item.BringRef`
  (params (Item :type "/Game/Object/BP_Items Object Reference") (Beer :type "/Game/Object/Nourriture/BP_Beer Object Reference"))
  (set `self.Item` Item))

(event `/Game/Blueprint/BPI_Input.RightTakes`
  (bind _item (`self.Item`))
  (bind _item_2 (`self.Item`))
  (if (not (`self.HoldingRight`))
    (`/Engine/EditorBlueprintResources/StandardMacros.IsValid` _item
      (:`Is Valid`
        (`self.Collisions` false)
        (if (`|EnumEquality` (`/Game/Object/BP_Items.TypeItem` _item) "NewEnumerator0")
          (`self.Biere`))
        (`self.K2_AttachToComponent` _item_2 (`self.CHR_Paw`) "Hand" "SnapToTarget" "KeepWorld" "KeepWorld" true)
        (`PrimitiveComponent.SetSimulatePhysics` (`/Game/Object/BP_Items.Item` _item_2) false)
        (set `self.HoldingRight` true)))))

(event `/Game/Blueprint/BPI_Input.RightReleases`
  (bind _item (`self.Item`))
  (if (`self.HoldingRight`)
    (`/Engine/EditorBlueprintResources/StandardMacros.IsValid` (`self.Item`)
      (:`Is Valid`
        (`self.K2_DetachFromActor` _item "KeepWorld" "KeepWorld" "KeepWorld")
        (`PrimitiveComponent.SetSimulatePhysics` (`/Game/Object/BP_Items.Item` _item) true)
        (bind _returnvalue (`KismetSystemLibrary.K2_SetTimerDelegate` (delegate `StopPhysic`) 0.4))))))

(event `StopPhysic`
  (`PrimitiveComponent.SetSimulatePhysics` (`/Game/Object/BP_Items.Item` (`self.Item`)) false)
  (`KismetSystemLibrary.K2_ClearAndInvalidateTimerHandle` (stale `/Game/Blueprint/BPI_Input.RightReleases` _returnvalue))
  (set `self.Item` (`self.VoidItem`))
  (set `self.HoldingRight` false)
  (message `/Game/Blueprint/BPI_Comm.RightCantTake` (`self.LeftPawn`))
  (`self.Collisions` true))

(event `self.ReceiveBeginPlay`
  (`TimelineComponent.SetPlayRate` (`self.GrabAnimation`) (/ 1.0 (`self.AnimDuration`)))
  (bind _asgm (cast `/Game/Blueprint/GM` (`GameplayStatics.GetGameMode`)))
  (set `self.GM` _asgm))

(event `/Game/Blueprint/BPI_Input.GrabAnim`
  (`/Engine/EditorBlueprintResources/StandardMacros.DoOnce` false :!label _label
    (:`Completed`
      (bind (_direction _alpha) (`Timeline|GrabAnimation` :!label _label_2)
        (:`Update`
          (`SkeletalMeshComponent.SetMorphTarget` (`self.CHR_Paw`) "paw_blendshape_02" (`KismetMathLibrary.Lerp` 0.0 1.0 _alpha) true))
        (:`Finished`
          (goto _label :!via `Reset`))))))

(event `/Game/Blueprint/BPI_Input.ReleaseAnim`
  (goto _label_2 :!via `Reverse`))

(event `Biere`
  (bind _returnvalue (`KismetMathLibrary.MakeTransform` (0.0 0.0 0.0)))
  (bind _alcoolbar (`/Game/Blueprint/GM.AlcoolBar` (`self.GM`)))
  (bind _output_get (set `/Game/Blueprint/Widget/WBP_AlcoolBar.currentAlcoolValue` (+ (`/Game/Blueprint/Widget/WBP_AlcoolBar.currentAlcoolValue` _alcoolbar) 0.333333) _alcoolbar))
  (if (<= _output_get 0.333333)
    (`|SpawnActorFromClass` "/Game/Blueprint/PostProcess/BP_PostProcessDrunked_lvl1.BP_PostProcessDrunked_lvl1_C" _returnvalue "Undefined" "MultiplyWithRoot" null null)
    (elif (<= _output_get 0.666667)
      (`|SpawnActorFromClass` "/Game/Blueprint/PostProcess/BP_PostProcessDrunked_lvl2.BP_PostProcessDrunked_lvl2_C" _returnvalue "Undefined" "MultiplyWithRoot" null null)
      (else
        (`|SpawnActorFromClass` "/Game/Blueprint/PostProcess/BP_PostProcessDrunked_lvl3.BP_PostProcessDrunked_lvl3_C" _returnvalue "Undefined" "MultiplyWithRoot" null null)))))

(fn `Collisions`
  (params (Collide :type Boolean))
  (bind _triger_main (`self.Triger Main`))
  (bind _chr_paw (`self.CHR_Paw`))
  (if Collide
    (`PrimitiveComponent.SetCollisionEnabled` _triger_main "QueryAndPhysics")
    (`PrimitiveComponent.SetCollisionEnabled` _chr_paw "QueryAndPhysics")
    (else
      (`PrimitiveComponent.SetCollisionEnabled` _triger_main "NoCollision")
      (`PrimitiveComponent.SetCollisionEnabled` _chr_paw "NoCollision"))))

(fn `SetClamp`
  (bind _returnvalue (`GameplayStatics.GetPlayerCameraManager` 1))
  (set `PlayerCameraManager.ViewPitchMin` 0.0 _returnvalue)
  (set `PlayerCameraManager.ViewPitchMax` 0.0 _returnvalue)
  (set `PlayerCameraManager.ViewYawMin` 0.0 _returnvalue)
  (set `PlayerCameraManager.ViewYawMax` 0.0 _returnvalue))

(fn `UserConstructionScript`)